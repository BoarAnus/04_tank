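; Player-drivable tank Blueprint with a turret, barrel, two tracks and a health bar widget.
; On BeginPlay it wires barrel and turret into the aiming component and tracks into the movement component, then gives the widget a self reference.
; Input drives tracks directly or through movement intents, and fires through the aiming component.
; Aim axes rotate a gimbal and spring arm scaled by delta time, and a toggle swaps between two cameras.
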(event `self.ReceiveBeginPlay`
  (`TankAimingComonent.Initialize` (`self.TankAimingComonent`) (`self.TankBarrel`) (`self.turret`))
  (`TankMovementComponent.Initialize` (`self.TankMovement`) (`self.LeftTankTrack`) (`self.RightTankTrack`))
  (`self.Initialise health bar widget`))

(event `InputAxis|Left Track Throttle`
  (params (AxisValue :type "Float (single-precision)"))
  ;[1 1 1] Movement
  (`TankTrack.SetThrottle` (`self.LeftTankTrack`) AxisValue))

(event `InputAxis|AimElevation`
  (params (AxisValue :type "Float (single-precision)"))
  ;[1 1 1] Aiming input binding
  (`SceneComponent.K2_AddLocalRotation` (`self.SpringArm`) (`KismetMathLibrary.MakeRotator` 0.0 (* AxisValue (`GameplayStatics.GetWorldDeltaSeconds`) 100.0)) false false))

(event `InputAxis|Right Track Throttle`
  (params (AxisValue :type "Float (single-precision)"))
  ;[1 1 1] Movement
  (`TankTrack.SetThrottle` (`self.RightTankTrack`) AxisValue))

(event `InputAxis|Throtlle Stick`
  (params (AxisValue :type "Float (single-precision)"))
  ;[1 1 1] Movement
  (`TankMovementComponent.IntendMoveFoward` (`self.TankMovement`) AxisValue))

(event `InputAxis|AimAzimuth`
  (params (AxisValue :type "Float (single-precision)"))
  ;[1 1 1] Aiming input binding
  (`SceneComponent.K2_AddLocalRotation` (`self.AzimuthGimble`) (`KismetMathLibrary.MakeRotator` 0.0 0.0 (* AxisValue (`GameplayStatics.GetWorldDeltaSeconds`) 100.0)) false false))

(event `InputAxis|Turn Stick`
  (params (AxisValue :type "Float (single-precision)"))
  ;[1 1 1] Movement
  (`TankMovementComponent.IntendTurn` (`self.TankMovement`) AxisValue))

(event `InputAction|Fire`
  (params (Key :type "Key Structure"))
  ;[1 1 1] Aiming input binding
  (:`Pressed`
    (`TankAimingComonent.FireTank` (`self.TankAimingComonent`))))

(event `InputAction|Toggle Camera`
  (params (Key :type "Key Structure"))
  ;[1 1 1] Camera swap
  (:`Pressed`
    (`ActorComponent.ToggleActive` (`self.Camera`))
    (`ActorComponent.ToggleActive` (`self.firstperson`))))

(fn `Initialise health bar widget`
  (bind _ashealth_bar (cast `/Game/UI/HealthBar` (`WidgetComponent.GetUserWidgetObject` (`self.Widget`))))
  (set `/Game/UI/HealthBar.My Tank` self _ashealth_bar)
  (return))

(fn `UserConstructionScript`)